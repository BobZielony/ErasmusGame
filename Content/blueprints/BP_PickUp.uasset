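; BP_PickUp is a pickup actor that the player collects by overlapping its Box component.
; An overlap by player character 0 increments PickCounterFromCharacer through ReferenceForCharacter, a character reference this graph never assigns.
; A DoOnce after the increment destroys the pickup and prints the new count.
; Colored debug strings report whether the overlapping actor is the player character.
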(event OnComponentBeginOverlap(Box)
  (params (OverlappedComponent :type Primitive%20Component%20Object%20Reference) (OtherActor :type Actor%20Object%20Reference) (OtherComp :type Primitive%20Component%20Object%20Reference) (OtherBodyIndex :type Integer) (bFromSweep :type Boolean) (SweepResult :type Hit%20Result%20Structure%20%28by%20ref%29))
  (bind _referenceforcharacter (Variables|Default|GetReferenceForCharacter))
  (if (== OtherActor (Game|GetPlayerCharacter 0))
    (Development|PrintString "This is the first person character" true true "(R=0.000000,G=1.000000,B=0.014447,A=1.000000)")
    (bind _output_get (Variables|/Game/FirstPerson/Blueprints/BP_FirstPersonCharacter.BP_FirstPersonCharacter_C|SetPickCounterFromCharacer _referenceforcharacter (+ (Variables|/Game/FirstPerson/Blueprints/BP_FirstPersonCharacter.BP_FirstPersonCharacter_C|GetPickCounterFromCharacer _referenceforcharacter) 1)))
    (Utilities|FlowControl|DoOnce false
      (:Completed
        (Actor|DestroyActor)
        (Development|PrintString (Utilities|String|ToString(Integer) _output_get))))
    (else
      (Development|PrintString "This is NOT the first person charcter" true true "(R=1.000000,G=0.024480,B=0.000000,A=1.000000)"))))

(fn ConstructionScript)