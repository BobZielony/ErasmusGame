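; BP_SmartSubstract is a box trigger that completes the macaroni pickup puzzle and moves the game on to Level_Kitchen.
; On overlap by BP_FirstPersonCharacter, it checks that the character's pickup counter equals exactly three.
; A match prints a completion message, plays an explosion sound and opens the level, otherwise it prints a pickup hint.
; Despite the name, the clamped counter-decrement logic is disconnected and never runs.
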(event OnComponentBeginOverlap(Box)
  (params (OverlappedComponent :type Primitive%20Component%20Object%20Reference) (OtherActor :type Actor%20Object%20Reference) (OtherComp :type Primitive%20Component%20Object%20Reference) (OtherBodyIndex :type Integer) (bFromSweep :type Boolean) (SweepResult :type Hit%20Result%20Structure%20%28by%20ref%29))
  (bind _asbp_first_person_character (Utilities|Casting|CastToBP_FirstPersonCharacter OtherActor))
  (if (== (Variables|/Game/FirstPerson/Blueprints/BP_FirstPersonCharacter.BP_FirstPersonCharacter_C|GetPickCounterFromCharacer _asbp_first_person_character) 3)
    (Development|PrintString "PUzzle complete")
    (Audio|PlaySound2D "/Game/StarterContent/Audio/Explosion01.Explosion01" 1.0 1.0 0.0 0 0)
    (Game|OpenLevel(byName) "Level_Kitchen")
    (else
      (Development|PrintString "You need to pickUp 3 macaroni"))))

(fn ConstructionScript)