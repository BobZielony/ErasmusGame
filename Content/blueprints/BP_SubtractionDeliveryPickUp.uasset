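; Pickup delivery Blueprint that checks whether the player character has collected exactly three pyramids, printing a door-opening win message or a request for more.
; A Gate node, driven by OpenTheGate and CloseTheGate, controls that check; OpenTheGate sends Enter before Open.
; On success the character's pickup counter becomes -1, but no door is actually moved here.
; The box overlap event is empty, and its player-check logic is disconnected.
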(event OnComponentBeginOverlap(Box)
  (params (OverlappedComponent :type Primitive%20Component%20Object%20Reference) (OtherActor :type Actor%20Object%20Reference) (OtherComp :type Primitive%20Component%20Object%20Reference) (OtherBodyIndex :type Integer) (bFromSweep :type Boolean) (SweepResult :type Hit%20Result%20Structure%20%28by%20ref%29)))

(event Custom|OpenTheGate
  (bind _referenceforcharacter (Variables|Default|GetReferenceForCharacter))
  (Development|PrintString "OpenTheGate")
  (Utilities|FlowControl|Sequence
    (:then_0
      (Utilities|FlowControl|Gate true :!label _label
        (:Exit
          (if (== (Variables|/Game/FirstPerson/Blueprints/BP_FirstPersonCharacter.BP_FirstPersonCharacter_C|GetPickCounterFromCharacer _referenceforcharacter) 3)
            (Development|PrintString "You win the door will open")
            (Variables|/Game/FirstPerson/Blueprints/BP_FirstPersonCharacter.BP_FirstPersonCharacter_C|SetPickCounterFromCharacer _referenceforcharacter -1)
            (else
              (Development|PrintString "You need more piramids"))))))
    (:then_1
      (goto _label Open))))

(event Custom|CloseTheGate
  (bind _referenceforcharacter (Variables|Default|GetReferenceForCharacter))
  (Utilities|FlowControl|Gate true) ; enters at Close
)

(fn ConstructionScript)