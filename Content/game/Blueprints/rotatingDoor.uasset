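; Door actor that opens only for a player who has the Jarzynowa flag set.
; When the first-person character overlaps the Box, the HasJarzynowa check decides the outcome.
; With the flag, the mesh snaps to a rotated yaw, then a DoOnce destroys the Box and shows the InformationToDeliver widget.
; Without it, a Jarzynowa widget is added to the viewport on each overlap.
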(event OnComponentBeginOverlap(Box)
  (params (OverlappedComponent :type Primitive%20Component%20Object%20Reference) (OtherActor :type Actor%20Object%20Reference) (OtherComp :type Primitive%20Component%20Object%20Reference) (OtherBodyIndex :type Integer) (bFromSweep :type Boolean) (SweepResult :type Hit%20Result%20Structure%20%28by%20ref%29))
  (bind _asbp_first_person_character (Utilities|Casting|CastToBP_FirstPersonCharacter OtherActor))
  (if (Variables|/Game/FirstPerson/Blueprints/BP_FirstPersonCharacter.BP_FirstPersonCharacter_C|GetHasJarzynowa _asbp_first_person_character)
    (Transformation|SetWorldRotation (Variables|Default|GetStaticMesh) "0.000000,-90.000000,0.000000" false false)
    (Utilities|FlowControl|DoOnce false
      (:Completed
        (Components|DestroyComponent (Variables|Default|GetBox))
        (bind _returnvalue (UserInterface|CreateWidget "/Game/game/Blueprints/InformationToDeliverWidget.InformationToDeliverWidget_C"))
        (UserInterface|Viewport|AddtoViewport _returnvalue 0)))
    (else
      (bind _returnvalue_2 (UserInterface|CreateWidget "/Game/game/Blueprints/JarzynowaWidget.JarzynowaWidget_C"))
      (UserInterface|Viewport|AddtoViewport _returnvalue_2 0))))

(event EventBeginPlay)

(event Collision|EventActorBeginOverlap
  (params (OtherActor :type Actor%20Object%20Reference)))

(event EventTick
  (params (DeltaSeconds :type Float%20%28single-precision%29)))

(fn ConstructionScript)