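; Exclamation mark marker actor that counts down the first-person character's TablesCounter when the player reaches it.
; When BP_FirstPersonCharacter overlaps the Box, it hides the Sphere and reveals StaticMesh1, including their children.
; A DoOnce then destroys the Box so it cannot retrigger, decrements the counter stored on the character and prints the new value.
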(event OnComponentBeginOverlap(Box)
  (params (OverlappedComponent :type Primitive%20Component%20Object%20Reference) (OtherActor :type Actor%20Object%20Reference) (OtherComp :type Primitive%20Component%20Object%20Reference) (OtherBodyIndex :type Integer) (bFromSweep :type Boolean) (SweepResult :type Hit%20Result%20Structure%20%28by%20ref%29))
  (bind _asbp_first_person_character (Utilities|Casting|CastToBP_FirstPersonCharacter OtherActor))
  (Development|SetHiddeninGame (Variables|Default|GetSphere) true true)
  (Development|SetHiddeninGame (Variables|Default|GetStaticMesh1) false true)
  (Utilities|FlowControl|DoOnce false
    (:Completed
      (Components|DestroyComponent (Variables|Default|GetBox))
      (bind _output_get (Variables|/Game/FirstPerson/Blueprints/BP_FirstPersonCharacter.BP_FirstPersonCharacter_C|SetTablesCounter _asbp_first_person_character (- (Variables|/Game/FirstPerson/Blueprints/BP_FirstPersonCharacter.BP_FirstPersonCharacter_C|GetTablesCounter _asbp_first_person_character) 1)))
      (Development|PrintString (Utilities|String|ToString(Integer) _output_get)))))

(event EventBeginPlay)

(event Collision|EventActorBeginOverlap
  (params (OtherActor :type Actor%20Object%20Reference)))

(event EventTick
  (params (DeltaSeconds :type Float%20%28single-precision%29)))

(fn ConstructionScript)