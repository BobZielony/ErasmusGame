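; BP_bucket is a bucket pickup that the first-person player collects by walking into it.
; When BP_FirstPersonCharacter overlaps the Box, it sets HasBucket on itself and HasBucketCharacter through its CHaracterReference variable, then prints a Polish pickup message.
; A DoOnce then destroys the mesh, handle, plane and trigger components, leaving the actor itself in place.
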(event OnComponentBeginOverlap(Box)
  (params (OverlappedComponent :type Primitive%20Component%20Object%20Reference) (OtherActor :type Actor%20Object%20Reference) (OtherComp :type Primitive%20Component%20Object%20Reference) (OtherBodyIndex :type Integer) (bFromSweep :type Boolean) (SweepResult :type Hit%20Result%20Structure%20%28by%20ref%29))
  (Utilities|Casting|CastToBP_FirstPersonCharacter OtherActor)
  (Variables|Default|SetHasBucket true)
  (Variables|/Game/FirstPerson/Blueprints/BP_FirstPersonCharacter.BP_FirstPersonCharacter_C|SetHasBucketCharacter (Variables|Default|GetCHaracterReference) true)
  (Development|PrintString "Podniosles wiadro")
  (Utilities|FlowControl|DoOnce false
    (:Completed
      (Components|DestroyComponent (Variables|Default|GetStaticMesh))
      (Components|DestroyComponent (Variables|Default|Getuszko))
      (Components|DestroyComponent (Variables|Default|GetPlane))
      (Components|DestroyComponent (Variables|Default|GetBox)))))

(fn ConstructionScript)