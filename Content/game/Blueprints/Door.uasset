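; Door actor that the player swings open and shut with the E key.
; A Timeline drives the SMDoor mesh's relative yaw at a fixed offset, playing forward when closed and reversing otherwise.
; Tick derives the closed state from the Timeline's current value.
; Box overlap enables player input, and the end-overlap event also calls EnableInput, so input is never disabled on leaving.
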(event OnComponentBeginOverlap(Box)
  (params (OverlappedComponent :type Primitive%20Component%20Object%20Reference) (OtherActor :type Actor%20Object%20Reference) (OtherComp :type Primitive%20Component%20Object%20Reference) (OtherBodyIndex :type Integer) (bFromSweep :type Boolean) (SweepResult :type Hit%20Result%20Structure%20%28by%20ref%29))
  (Input|EnableInput (Game|GetPlayerController 0)))

(event OnComponentEndOverlap(Box)
  (params (OverlappedComponent :type Primitive%20Component%20Object%20Reference) (OtherActor :type Actor%20Object%20Reference) (OtherComp :type Primitive%20Component%20Object%20Reference) (OtherBodyIndex :type Integer))
  (Input|EnableInput (Game|GetPlayerController 0)))

(event EventTick
  (params (DeltaSeconds :type Float%20%28single-precision%29))
  (Variables|Default|SetDoorClosed (< (stale Input|KeyboardEvents|E _door) 1.0)))

(event Input|KeyboardEvents|E
  (params (Key :type Key%20Structure :default "None"))
  (:Pressed
    (if (Variables|Default|GetDoorClosed)
      (bind _door (Timeline|Timeline Play)
        (:Update
          (Transformation|SetRelativeLocationAndRotation (Variables|Default|GetSM_Door) "0.000000,45.468759,0.000000" (Math|Rotator|MakeRotator 0.0 0.0 _door) false false)))
      (else
        (Timeline|Timeline Reverse)))))

(fn ConstructionScript)